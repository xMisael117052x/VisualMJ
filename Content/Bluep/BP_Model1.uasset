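; BP_Model1 is an actor that swaps the material on its static mesh when Q is pressed.
; It enables player input on BeginPlay, and each press advances a MultiGate through six preset materials in fixed order.
; Each step applies a new dynamic material instance to element 0.
; The gate does not loop, so presses after the sixth change nothing.
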(event EventBeginPlay
  (Input|EnableInput (Game|GetPlayerController 0)))

(event Input|KeyboardEvents|Q
  (params (Key :type Key%20Structure :default "None"))
  (:Pressed
    (Utilities|FlowControl|MultiGate false false -1
      (:Out%200
        (Rendering|Material|CreateDynamicMaterialInstance (Variables|Default|GetStaticMesh) 0 "/Engine/VREditor/UI/FrameMaterial.FrameMaterial" "None" :!class /Script/Engine.PrimitiveComponent))
      (:Out%201
        (Rendering|Material|CreateDynamicMaterialInstance (Variables|Default|GetStaticMesh) 0 "/Game/Fab/WUD_Chess_Piece_Queen/Material_1.Material_1" "None" :!class /Script/Engine.PrimitiveComponent))
      (:Out%202
        (Rendering|Material|CreateDynamicMaterialInstance (Variables|Default|GetStaticMesh) 0 "/Game/PortalMaterial/Material/M_Wisp_Inst.M_Wisp_Inst" "None" :!class /Script/Engine.PrimitiveComponent))
      (:Out%203
        (Rendering|Material|CreateDynamicMaterialInstance (Variables|Default|GetStaticMesh) 0 "/Engine/MapTemplates/Materials/BasicTemplateMaterial.BasicTemplateMaterial" "None" :!class /Script/Engine.PrimitiveComponent))
      (:Out%204
        (Rendering|Material|CreateDynamicMaterialInstance (Variables|Default|GetStaticMesh) 0 "/Engine/EngineMeshes/BackgroundMaterial.BackgroundMaterial" "None" :!class /Script/Engine.PrimitiveComponent))
      (:Out%205
        (Rendering|Material|CreateDynamicMaterialInstance (Variables|Default|GetStaticMesh) 0 "/Engine/EngineDebugMaterials/HeatmapMaterial.HeatmapMaterial" "None" :!class /Script/Engine.PrimitiveComponent)))))

(fn ConstructionScript)