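; BP_Vis is a controllable camera pawn with a spring arm that supports look and zoom through Enhanced Input.
; BeginPlay aligns control rotation to the camera, lets the arm follow it, sets ViewPitchMax twice (never ViewPitchMin), and enables the cursor with Game and UI input.
; Look feeds controller yaw and adds pitch both positive and negated, cancelling it out.
; Zoom offsets arm length by scaled input, without clamping.
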(event Input|EnhancedActionEvents|EnhancedInputActionZoom
  (params (ActionValue :type Float%20%28double-precision%29) (ElapsedSeconds :type Float%20%28double-precision%29) (TriggeredSeconds :type Float%20%28double-precision%29) (InputAction :type Input%20Action%20Object%20Reference :default "/Game/Bluep/Zoom.Zoom"))
  (bind _springarm (Variables|Default|GetSpringArm))
  (Variables|/Script/Engine.SpringArmComponent|SetTargetArmLength _springarm (+ (* ActionValue 6e+01) (Variables|/Script/Engine.SpringArmComponent|GetTargetArmLength _springarm))))

(event Input|EnhancedActionEvents|EnhancedInputActionIA_Look
  (params (ActionValue :type Vector%202D%20Structure) (ElapsedSeconds :type Float%20%28double-precision%29) (TriggeredSeconds :type Float%20%28double-precision%29) (InputAction :type Input%20Action%20Object%20Reference :default "/Game/ThirdPerson/Input/Actions/IA_Look.IA_Look"))
  (Pawn|Input|AddControllerYawInput (.x ActionValue))
  (Pawn|Input|AddControllerPitchInput (.y ActionValue))
  (Pawn|Input|AddControllerPitchInput (* (.y ActionValue) -1.0)))

(event EventBeginPlay
  (bind _returnvalue (Game|GetPlayerController 0))
  (bind _returnvalue_2 (Game|GetPlayerController 0))
  (bind _playercameramanager (Variables|/Script/Engine.PlayerController|GetPlayerCameraManager _returnvalue))
  (Pawn|SetControlRotation (Game|GetPlayerController 0) (Transformation|GetWorldRotation (Variables|Default|GetCamera)))
  (Variables|/Script/Engine.SpringArmComponent|SetbUsePawnControlRotation (Variables|Default|GetSpringArm) true)
  (Variables|/Script/Engine.PlayerCameraManager|SetViewPitchMax _playercameramanager -8e+01)
  (Variables|/Script/Engine.PlayerCameraManager|SetViewPitchMax _playercameramanager -3e+01)
  (Variables|/Script/Engine.PlayerController|SetbShowMouseCursor _returnvalue_2 true)
  (Input|SetInputModeGameandUI _returnvalue_2 0 "DoNotLock" true false))

(fn ConstructionScript)